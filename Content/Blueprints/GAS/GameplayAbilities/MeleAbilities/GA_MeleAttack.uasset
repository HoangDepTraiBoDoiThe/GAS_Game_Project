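; GA_MeleAttack is a melee attack gameplay ability that plays the AM_Attack montage and ends when it completes, is interrupted or is cancelled.
; On the Montage.Attack gameplay event, it starts motion warping toward the avatar's current target through CombatInterface.
; It then runs a sphere hit check at the weapon location, ignoring the avatar, and applies a gameplay effect to each hit actor not on the same team.
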(event Ability|EventActivateAbility
  (bind _returnvalue (Ability|GetAvatarActorfromActorInfo))
  (|PlayMontageandWaitProxy "None" "/Game/Blueprints/Characters/Enemies/Mele/AM_Attack.AM_Attack" 1.0 "None" true 1.0 0.0 false
    (:then
      (Ability|Tasks|WaitGameplayEvent "(TagName=\"Montage.Attack\")" 0
        (:EventReceived
          (bind _ascombat_interface (Utilities|Casting|CastToCombatInterface (Ability|GetAvatarActorfromActorInfo)))
          (bind _returnvalue_2 (Class|CombatInterface|GetCurTarget _ascombat_interface))
          (Class|CombatInterface|StartMotionWarping _ascombat_interface (Transformation|GetActorLocation _returnvalue_2))
          (bind _returnvalue_3 (Class|CombatInterface|WeaponLocation _ascombat_interface))
          (bind _overlaptargetactors (Class|DamageGameplayAbility|MakeSphereHitChecker _returnvalue (Utilities|Array|MakeArray _returnvalue) _returnvalue _returnvalue_3 (Variables|Default|GetSphereRadius)))
          (for _array_element _overlaptargetactors
            (if (not (Class|MyBlueprintFunctionLibrary|AreWeonintheSameTeam _array_element (Ability|GetAvatarActorfromActorInfo)))
              (Class|DamageGameplayAbility|AppliedMyGameplayEffecttoTarget (Ability|GetAbilitySystemComponent _array_element)))))))
    (:OnCompleted
      (Ability|EndAbility :!label _label))
    (:OnInterrupted
      (goto _label))
    (:OnCancelled
      (goto _label))))

(event Ability|EventOnEndAbility
  (params (bWasCancelled :type Boolean)))