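; Gameplay ability that plays a hit reaction on its avatar while a GE_HitReact effect is active.
; On activation it applies the effect to the avatar's ability system component and stores the handle, then gets the montage through CombatInterface, keeping the ability character-agnostic.
; When the montage completes, is interrupted or is cancelled, it removes the effect by that handle and ends the ability.
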(event Ability|EventActivateAbility
  (bind _returnvalue (GameplayEffects|ApplyGameplayEffectToSelf :self (Ability|GetAbilitySystemComponent (Ability|GetAvatarActorfromActorInfo)) :GameplayEffectClass "/Game/Blueprints/GAS/GameplayEffects/GE_HitReact.GE_HitReact_C"))
  (Variables|Default|SetHitReactGameplayEffectHandle _returnvalue)
  (bind _ascombat_interface (Utilities|Casting|CastToCombatInterface (Ability|GetAvatarActorfromActorInfo)))
  (bind _returnvalue_2 (Class|CombatInterface|GetHitReactMontage _ascombat_interface))
  (|PlayMontageandWaitProxy "None" _returnvalue_2 1.0 "None" true 1.0 0.0 false
    (:OnCompleted
      _)
    (:OnInterrupted
      _)
    (:OnCancelled
      _))
  (Ability|RemoveGameplayEffectFromOwnerWithHandle (Variables|Default|GetHitReactGameplayEffectHandle))
  (Ability|EndAbility))

(event Ability|EventOnEndAbility
  (params (bWasCancelled :type Boolean)))