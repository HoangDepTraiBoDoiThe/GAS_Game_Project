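; Behavior tree task that triggers an AI pawn's elemental attack ability, gated by its minion count.
; On AI tick, it passes the blackboard target to the pawn's combat interface and reads its minion count and threshold.
; While the count is below the threshold, it activates abilities matching a tag container through the pawn's Ability System Component.
; It succeeds whenever the target is valid, even without activating, and fails otherwise.
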(event EventReceiveTickAI
  (params (OwnerController :type AI%20Controller%20Object%20Reference) (ControlledPawn :type Pawn%20Object%20Reference) (DeltaSeconds :type Float%20%28single-precision%29))
  (Variables|Default|SetControlledPawn ControlledPawn)
  (bind _ascombat_interface (Utilities|Casting|CastToCombatInterface ControlledPawn))
  (Variables|Default|SettargetActor (AI|BehaviorTree|GetBlackboardValueasActor (Variables|Default|GetTarget)))
  (Utilities|IsValid (Variables|Default|GettargetActor)
    (:Is%20Valid
      (Class|CombatInterface|SetCurTarget _ascombat_interface (Variables|Default|GettargetActor))
      (bind _returnvalue (Class|CombatInterface|GetMinionMinionCount(Message) (Variables|Default|GetControlledPawn)))
      (Variables|Default|SetMinionCount _returnvalue)
      (bind _returnvalue_2 (Class|CombatInterface|GetMinionThreadHold(Message) (Variables|Default|GetControlledPawn)))
      (Variables|Default|SetMinionThreadHold _returnvalue_2)
      (if (< (Variables|Default|GetMinionCount) (Variables|Default|GetMinionThreadHold))
        (Abilities|TryActivateAbilitiesbyTag (Ability|GetAbilitySystemComponent (Variables|Default|GetControlledPawn)) (Variables|Default|GetAbility%20tags) true))
      (AI|BehaviorTree|FinishExecute true))
    (:Is%20Not%20Valid
      (AI|BehaviorTree|FinishExecute false))))